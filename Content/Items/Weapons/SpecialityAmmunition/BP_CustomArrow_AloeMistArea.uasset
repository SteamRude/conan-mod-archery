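; Area effect actor for the Aloe mist custom arrow that applies a configured buff to players and thralls inside it.
; On the server, sphere overlaps track characters, and a looping timer reapplies stacks through their buff system components.
; Leaving removes the stacks unless the effect lingers.
; After a short delay, a timer shrinks the particles and trigger sphere until the actor destroys itself.
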(event `self.Trigger Sphere.OnComponentBeginOverlap`
  (params (OverlappedComponent :type "PrimitiveComponent Object Reference") (OtherActor :type "Actor Object Reference") (OtherComp :type "PrimitiveComponent Object Reference") (OtherBodyIndex :type Integer) (bFromSweep :type Boolean) (SweepResult :type "HitResult Structure (by ref)"))
  (bind _asconan_character (cast `ConanCharacter` OtherActor))
  (if (or (`ConanCharacter.IsThrall` _asconan_character) (`ConanCharacter.IsPlayer` _asconan_character))
    (`self.Player Enters` _asconan_character)
    (`self.Apply Buff` _asconan_character)))

(event `self.Trigger Sphere.OnComponentEndOverlap`
  (params (OverlappedComponent :type "PrimitiveComponent Object Reference") (OtherActor :type "Actor Object Reference") (OtherComp :type "PrimitiveComponent Object Reference") (OtherBodyIndex :type Integer))
  (bind _asconan_character (cast `ConanCharacter` OtherActor))
  (if (or (`ConanCharacter.IsThrall` _asconan_character) (`ConanCharacter.IsPlayer` _asconan_character))
    (`self.Player Leaves` _asconan_character)
    (if (not (`self.Lingering Debuff ?`))
      (`self.Remove Buff` _asconan_character))))

(event `Player Enters`
  (params (Player :type "Actor Object Reference"))
  (`KismetArrayLibrary.Array_Insert` (`self.Affected Chars`) Player)
  (if (not (`KismetSystemLibrary.K2_TimerExistsHandle` (`self.TimerHandle`)))
    (bind _returnvalue (`KismetSystemLibrary.K2_SetTimerDelegate` (delegate `Hazard Tick`) (`self.Tick Time`) true))
    (set `self.TimerHandle` _returnvalue)))

(event `Hazard Tick`
  (for _array_element (`self.Affected Chars`)
    (`self.Apply Buff` _array_element)))

(event `Player Leaves`
  (params (Player :type "Actor Object Reference"))
  (`KismetArrayLibrary.Array_RemoveItem` (`self.Affected Chars`) Player))

(event `self.ReceiveBeginPlay`
  (`parent.ReceiveBeginPlay`)
  (`KismetSystemLibrary.K2_SetTimerDelegate` (delegate `Start Timer`) 5.0)
  (if (not (`KismetSystemLibrary.IsServer`))
    (`ActorComponent.K2_DestroyComponent` (`self.Trigger Sphere`))))

(event `Start Timer`
  (`KismetSystemLibrary.K2_SetTimerDelegate` (delegate `Fadeout`) 0.1 true))

(event `Fadeout`
  (bind _output_get (set `self.Scale` (- (`self.Scale`) (0.01 0.01 0.01))))
  (`SceneComponent.SetRelativeScale3D` (`self.ParticleSystem`) _output_get)
  (bind _output_get_2 (set `self.Radius` (- (`self.Radius`) 2.0)))
  (`SphereComponent.SetSphereRadius` (`self.Trigger Sphere`) _output_get_2 true)
  (if (== _output_get (0.0 0.0 0.0))
    (`self.K2_DestroyActor`)))

(fn `Apply Buff`
  (params (Player :type "Actor Object Reference"))
  (bind _returnvalue (`self.K2_GetComponentsByClass` Player "/Game/Systems/Buffs/00_BP_AC_BuffSystem.00_BP_AC_BuffSystem_C"))
  (if (>= (`KismetArrayLibrary.Array_Length` _returnvalue) 0)
    (for _ (range 1 (+ (`self.Stacks`) 1))
      (`/Game/Systems/Buffs/00_BP_AC_BuffSystem.AddBuff` (`KismetArrayLibrary.Array_Get` _returnvalue) (`self.Hazard Debuff`) (`self.Potency`) (`Pawn.GetController` (`self.Instigator`))))))

(fn `DoTick`)

(fn `Remove Buff`
  (params (Player :type "Actor Object Reference"))
  (bind _returnvalue (`self.K2_GetComponentsByClass` Player "/Game/Systems/Buffs/00_BP_AC_BuffSystem.00_BP_AC_BuffSystem_C"))
  (if (>= (`KismetArrayLibrary.Array_Length` _returnvalue) 0)
    (for _ (range 1 (+ (`self.Stacks`) 1))
      (`/Game/Systems/Buffs/00_BP_AC_BuffSystem.RemoveBuff` (`KismetArrayLibrary.Array_Get` _returnvalue) (`self.Hazard Debuff`)))))

(fn `UserConstructionScript`)